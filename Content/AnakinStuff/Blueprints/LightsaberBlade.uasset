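; Lightsaber blade actor that damages battle droids it touches.
; Each tick it scans its overlapping components for the DroidBody tag and disables its own tick on a match, with no re-enable in this Blueprint.
; It casts the component's owner to Battledroid and, if that droid still has health, calls DecreaseHealth, plays a hit sound at the blade and stops scanning.
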(event EventTick
  (params (DeltaSeconds :type Float%20%28single-precision%29))
  (bind _array_element (Utilities|Array|ForEachLoopwithBreak (Class|Actor|GetOverlappingComponents) :!label _label)
    (:LoopBody
      (if (Components|ComponentHasTag _array_element "DroidBody")
        (Actor|Tick|SetActorTickEnabled false)
        (bind _asbattledroid (Utilities|Casting|CastToBattledroid (Components|GetOwner _array_element)))
        (if (not (<= (Variables|/Game/Battledroids/Super_Battledroid/Battledroid.Battledroid_C|GetHealth _asbattledroid) 0.0))
          (Default|DecreaseHealth _asbattledroid)
          (Audio|PlaySoundatLocation "/Game/AnakinStuff/Audio/Lightsaber_Sounds/HitSounds.HitSounds" (Transformation|GetActorLocation) "0, 0, 0" 1.0 1.0 0.0 0 0 0 0)
          (goto _label Break))))))

(fn ConstructionScript)